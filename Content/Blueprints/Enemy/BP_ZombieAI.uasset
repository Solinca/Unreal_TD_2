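; Zombie enemy that signals when to chase the player and reacts to landing attacks, taking damage and dying.
; It binds to its AI controller's player-hit event, fires ChasePlayer shortly after spawn, and fires it again after each attack.
; HealthComponent events drive hit reactions and death, which fires TriggerDeath, disables capsule collision and destroys the actor.
; Animations play directly on the mesh, sequenced with fixed delays.
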(event OnHealthDepleted(HealthComponent)
  ;[0.15 0.15 0.15 0.5] Trigger Zombie Death
  (Default|CallTriggerDeath)
  (Variables|Default|SetIsDead true)
  (Collision|SetCollisionEnabled (Variables|Default|GetCapsuleComponent) "NoCollision")
  (Components|Animation|PlayAnimation (Variables|Character|GetMesh) "/Game/Assets/ZombieAnimationPack/Animations/anim_Burst_C.anim_Burst_C" false)
  (Utilities|FlowControl|Delay 1.5)
  (Actor|DestroyActor))

(event OnHealthChanged(HealthComponent)
  (params (CurrentHealth :type Integer) (MaxHealth :type Integer))
  ;[0.15 0.15 0.15 0.5] Play Hit Damage Anim
  (if (not (or (== CurrentHealth MaxHealth) (<= CurrentHealth 0)))
    (Components|Animation|PlayAnimation (Variables|Character|GetMesh) "/Game/Assets/ZombieAnimationPack/Animations/anim_Taking_Damage_F.anim_Taking_Damage_F" false)
    (Utilities|FlowControl|Delay 0.8)
    (if (not (Variables|Default|GetIsDead))
      (Components|Animation|PlayAnimation (Variables|Character|GetMesh) "/Game/Assets/ZombieAnimationPack/Animations/anim_Walk_B.anim_Walk_B" false))))

(event Custom|TriggerPlayerHit_Event
  ;[0.15 0.15 0.15 0.5] Bind Trigger Player Hit Event
  ;[0.15 0.15 0.15 0.5] Play Attack Animation and Chase Player at the end of it
  (Components|Animation|PlayAnimation (Variables|Default|GetMesh) "/Game/Assets/ZombieAnimationPack/Animations/anim_Attack_A.anim_Attack_A" false)
  (Utilities|FlowControl|Delay 0.7)
  (Components|Animation|PlayAnimation (Variables|Default|GetMesh) "/Game/Assets/ZombieAnimationPack/Animations/anim_Walk_B.anim_Walk_B" false)
  (Default|CallChasePlayer))

(event EventBeginPlay
  ;[0.15 0.15 0.15 0.5] Bind Trigger Player Hit Event
  (bind _asaic_zombie_aicontroller (Utilities|Casting|CastToAIC_ZombieAIController (Pawn|GetController)))
  (EventDispatchers|AssignTriggerPlayerHit _asaic_zombie_aicontroller (delegate Custom|TriggerPlayerHit_Event))
  ;[0.15 0.15 0.15 0.5] First call to chase
  (Utilities|FlowControl|Delay 0.01)
  (Default|CallChasePlayer))

(fn ConstructionScript)