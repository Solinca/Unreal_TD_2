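; Player character Blueprint that ties health and weapon components to the character and re-broadcasts their events.
; Health depletion, health change and ammo change events are forwarded through the character's own dispatchers.
; A weapon switch sets the weapon mesh from the weapon data and attaches it to that data's socket on the character mesh.
; The X key applies test damage, and the weapon-shot event is an empty stub.
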(event OnWeaponSwitched(PlayerWeaponComponent)
  (params (WeaponData :type Weapon%20Data%20Structure))
  (bind (_weaponmesh _weaponsocket) (Utilities|Struct|BreakWeaponData WeaponData))
  ;[0.15 0.15 0.15 0.5] Switch Weapon Model OnWeaponSwitched
  (Components|StaticMesh|SetStaticMesh (Variables|Default|GetPlayerWeaponMesh) _weaponmesh)
  (Transformation|AttachComponentToComponent (Variables|Default|GetPlayerWeaponMesh) (Variables|Character|GetMesh) _weaponsocket "KeepRelative" "KeepRelative" "KeepRelative" true))

(event OnWeaponShot(PlayerWeaponComponent))

(event OnHealthDepleted(PlayerHealthComponent)
  ;[0.15 0.15 0.15 0.5] Forward OnHealthDepleted Event
  (Default|CallOnHealthDepleted))

(event OnHealthChanged(PlayerHealthComponent)
  (params (CurrentHealth :type Integer) (MaxHealth :type Integer))
  ;[0.15 0.15 0.15 0.5] Forward OnHealthChanged Event
  (Default|CallOnHealthChanged CurrentHealth MaxHealth))

(event OnWeaponAmmoChanged(PlayerWeaponComponent)
  (params (CurrentAmmo :type Integer) (MaxAmmo :type Integer))
  ;[0.15 0.15 0.15 0.5] Forward OnWeaponAmmoChanged
  (Default|CallOnWeaponAmmoChanged CurrentAmmo MaxAmmo))

(event Input|KeyboardEvents|X
  (params (Key :type Key%20Structure :default "None"))
  ;[0.15 0.15 0.15 0.5] Simulate taking one damage with "X"
  (:Pressed
    (Class|PlayerHealthComponent|TakeDamage (Variables|Default|GetPlayerHealthComponent) 1)))

(fn ConstructionScript)