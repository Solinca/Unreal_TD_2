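; Player controller that owns the player HUD, wave round and pause widgets.
; On BeginPlay it creates the widgets, shows the HUD and forwards the character's health and weapon ammo change events to it.
; P pauses the game with UI-only input until the pause widget's resume event restores play.
; L is a test key that briefly shows the wave round widget.
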(event Custom|ResumeGameEvent_Event
  ;[0.15 0.15 0.15 0.5] React to "Resume Game" button press
  (Widget|RemovefromParent (Variables|Default|GetPauseUI))
  (Game|SetGamePaused false)
  (Variables|Default|SetbShowMouseCursor false)
  (Input|SetInputModeGameOnly self false))

(event Custom|OnHealthChanged_Event
  (params (Current%20Health :type Integer) (Max%20Health :type Integer))
  ;[0.15 0.15 0.15 0.5] Forward OnHealthChanged to UI
  (Default|SetPlayerHealth (Variables|Default|GetPlayerUI) Current%20Health Max%20Health))

(event Custom|OnWeaponAmmoChanged_Event
  (params (Current%20Ammo :type Integer) (Max%20Ammo :type Integer))
  ;[0.15 0.15 0.15 0.5] Forward OnWeaponAmmoChanged to UI
  (Default|SetPlayerAmmo (Variables|Default|GetPlayerUI) Current%20Ammo Max%20Ammo))

(event EventBeginPlay
  ;[0.15 0.15 0.15 0.5] Create Player UI and add it to screen
  (bind _returnvalue (UserInterface|CreateWidget "/Game/Blueprints/WidgetBlueprints/WBP_PlayerUI.WBP_PlayerUI_C"))
  (bind _output_get (Variables|Default|SetPlayerUI _returnvalue))
  (UserInterface|Viewport|AddtoViewport _output_get 0)
  ;[0.15 0.15 0.15 0.5] Create Wave Round UI and set it as parameter
  (bind _returnvalue_2 (UserInterface|CreateWidget "/Game/Blueprints/WidgetBlueprints/WBP_WaveRoundUI.WBP_WaveRoundUI_C"))
  (Variables|Default|SetWaveUI _returnvalue_2)
  ;[0.15 0.15 0.15 0.5] Create Pause UI and set it as parameter
  (bind _returnvalue_3 (UserInterface|CreateWidget "/Game/Blueprints/WidgetBlueprints/WBP_PauseUI.WBP_PauseUI_C"))
  (Variables|Default|SetPauseUI _returnvalue_3)
  ;[0.15 0.15 0.15 0.5] Forward OnHealthChanged to UI
  (bind _asbp_my_character (Utilities|Casting|CastToBP_MyCharacter (Game|Player|GetPlayerPawn 0)))
  (EventDispatchers|AssignOnHealthChanged _asbp_my_character (delegate Custom|OnHealthChanged_Event))
  ;[0.15 0.15 0.15 0.5] Forward OnWeaponAmmoChanged to UI
  (EventDispatchers|AssignOnWeaponAmmoChanged _asbp_my_character (delegate Custom|OnWeaponAmmoChanged_Event)))

(event Input|KeyboardEvents|P
  (params (Key :type Key%20Structure :default "None"))
  ;[0.15 0.15 0.15 0.5] Pause game when pressing "P"
  (:Pressed
    (UserInterface|Viewport|AddtoViewport (Variables|Default|GetPauseUI) 0)
    (Game|SetGamePaused true)
    (Variables|Default|SetbShowMouseCursor true)
    (Input|SetInputModeUIOnly self 0 "DoNotLock" false)
    ;[0.15 0.15 0.15 0.5] React to "Resume Game" button press
    (EventDispatchers|AssignResumeGameEvent (Variables|Default|GetPauseUI) (delegate Custom|ResumeGameEvent_Event))))

(event Input|KeyboardEvents|L
  (params (Key :type Key%20Structure :default "None"))
  ;[0.15 0.15 0.15 0.5] Test Wave Launch with delay by pressing "L"
  (:Pressed
    (UserInterface|Viewport|AddtoViewport (Variables|Default|GetWaveUI) 0)
    (Utilities|FlowControl|Delay 4.0)
    (Widget|RemovefromParent (Variables|Default|GetWaveUI))))

(fn ConstructionScript)